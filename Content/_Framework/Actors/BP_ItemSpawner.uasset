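; BP_ItemSpawner is an actor that scatters blue, red, green and yellow item actors inside a spawn area.
; SpawnItems reads per-color tool amounts from GS_Case and spawns each at a random point in a fixed-size volume centered on the Box component, adjusting for collisions but always spawning.
; SR_SpawnItems only calls MCSpawnItems; MC_SpawnItems is empty, and nothing in this graph calls SpawnItems.
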(event `self.ReceiveBeginPlay`
  (`parent.ReceiveBeginPlay`))

(event `SR_SpawnItems`
  ;[1 1 1] Spawn Items in the spawn area.
  (`self.MC_SpawnItems`))

(event `MC_SpawnItems`
  ;[1 1 1] Spawn Items in the spawn area.
)

(event `SpawnItems`
  ;[1 1 1] Spawn Items in the spawn area.
  (bind _asgs_case (cast `/Game/_Framework/Blueprints/GS_Case` (`GameplayStatics.GetGameState`)))
  (for _ (range 1 (+ (`/Game/_Framework/Blueprints/GS_Case.BlueToolAmount` _asgs_case) 1))
    (`|SpawnActorFromClass` "/Game/_Framework/Actors/BP_ItemBlue.BP_ItemBlue_C" (`KismetMathLibrary.MakeTransform` (`KismetMathLibrary.RandomPointInBoundingBox` (`SceneComponent.K2_GetComponentLocation` (`self.Box`)) (300.0 300.0 150.0))) "AdjustIfPossibleButAlwaysSpawn" "MultiplyWithRoot" null null))
  (for _ (range 1 (+ (`/Game/_Framework/Blueprints/GS_Case.RedToolAmount` _asgs_case) 1))
    (`|SpawnActorFromClass` "/Game/_Framework/Actors/BP_ItemRed.BP_ItemRed_C" (`KismetMathLibrary.MakeTransform` (`KismetMathLibrary.RandomPointInBoundingBox` (`SceneComponent.K2_GetComponentLocation` (`self.Box`)) (300.0 300.0 150.0))) "AdjustIfPossibleButAlwaysSpawn" "MultiplyWithRoot" null null))
  (for _ (range 1 (+ (`/Game/_Framework/Blueprints/GS_Case.GreenToolAmount` _asgs_case) 1))
    (`|SpawnActorFromClass` "/Game/_Framework/Actors/BP_ItemGreen.BP_ItemGreen_C" (`KismetMathLibrary.MakeTransform` (`KismetMathLibrary.RandomPointInBoundingBox` (`SceneComponent.K2_GetComponentLocation` (`self.Box`)) (300.0 300.0 150.0))) "AdjustIfPossibleButAlwaysSpawn" "MultiplyWithRoot" null null))
  (for _ (range 1 (+ (`/Game/_Framework/Blueprints/GS_Case.YellowToolAmount` _asgs_case) 1))
    (`|SpawnActorFromClass` "/Game/_Framework/Actors/BP_ItemYellow.BP_ItemYellow_C" (`KismetMathLibrary.MakeTransform` (`KismetMathLibrary.RandomPointInBoundingBox` (`SceneComponent.K2_GetComponentLocation` (`self.Box`)) (300.0 300.0 150.0))) "AdjustIfPossibleButAlwaysSpawn" "MultiplyWithRoot" null null)))

(fn `UserConstructionScript`
  (`parent.UserConstructionScript`))