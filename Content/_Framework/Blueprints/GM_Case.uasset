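; GM_Case is the game mode that tracks connected players and starts a match.
; PostLogin and OnLogout maintain PlayerList, and SR_CommenceGame passes the start to MC_CommenceGame.
; That event moves each player's pawn to a random point inside the BP_PlayerTeleportLocation box and triggers BP_ItemSpawner.
; It then loops over PlayerList to hide the cursor, set game-only input and call CommenceGame on each HUD_Case.
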(event `self.K2_PostLogin`
  (params (NewPlayer :type "PlayerController Object Reference"))
  (`KismetArrayLibrary.Array_Add` (`self.PlayerList`) NewPlayer))

(event `self.K2_OnLogout`
  (params (ExitingController :type "Controller Object Reference"))
  (`KismetArrayLibrary.Array_RemoveItem` (`self.PlayerList`) (`PlayerState.GetPlayerController` (`Controller.PlayerState` ExitingController))))

(event `SR_CommenceGame`
  (`self.MC_CommenceGame`))

(event `MC_CommenceGame`
  (`self.TeleportPlayers`)
  (`self.SpawnItems`)
  (`self.UpdateUISettings`))

(event `TeleportPlayers`
  (bind _returnvalue (`GameplayStatics.GetActorOfClass` "/Game/_Framework/Actors/BP_PlayerTeleportLocation.BP_PlayerTeleportLocation_C"))
  (for _array_element (`self.PlayerList`)
    (bind (_origin _boxextent) (`KismetSystemLibrary.GetComponentBounds` (`/Game/_Framework/Actors/BP_SpawnAreaBase.Box` _returnvalue)))
    (`self.K2_SetActorLocation` (`Controller.K2_GetPawn` _array_element) (`KismetMathLibrary.RandomPointInBoundingBox` _origin _boxextent) false false)))

(event `SpawnItems`
  (bind _returnvalue (`GameplayStatics.GetActorOfClass` "/Game/_Framework/Actors/BP_ItemSpawner.BP_ItemSpawner_C"))
  (`/Game/_Framework/Actors/BP_ItemSpawner.SpawnItems` _returnvalue))

(event `UpdateUISettings`
  (for _array_element (`self.PlayerList`)
    (set `PlayerController.bShowMouseCursor` false _array_element)
    (`WidgetBlueprintLibrary.SetInputMode_GameOnly` _array_element)
    (bind _ashud_case (cast `/Game/_Framework/HUD_Case` (`PlayerController.GetHUD` _array_element)))
    (`/Game/_Framework/HUD_Case.CommenceGame` _ashud_case)))

(fn `UserConstructionScript`)