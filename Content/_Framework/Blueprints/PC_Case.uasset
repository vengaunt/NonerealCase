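; Player controller for the Case game mode that shows the mouse cursor and increments shared tool counts in four colors.
; On BeginPlay it caches the GS_Case game state, which holds the blue, red, green and yellow tool amounts.
; Each color has an SR_ event that calls an MC_ event, named as a server-to-multicast relay, which increments that color's count on the game state.
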(event `self.ReceiveBeginPlay`
  (set `self.bShowMouseCursor` true)
  (bind _asgs_case (cast `/Game/_Framework/Blueprints/GS_Case` (`GameplayStatics.GetGameState`)))
  (set `self.GS` _asgs_case))

(event `SR_AddBlue`
  (`self.MC_AddBlue`))

(event `MC_AddBlue`
  (`/Engine/EditorBlueprintResources/StandardMacros.IncrementInt` (`/Game/_Framework/Blueprints/GS_Case.BlueToolAmount` (`self.GS`))))

(event `SR_AddRed`
  (`self.MC_AddRed`))

(event `MC_AddRed`
  (`/Engine/EditorBlueprintResources/StandardMacros.IncrementInt` (`/Game/_Framework/Blueprints/GS_Case.RedToolAmount` (`self.GS`))))

(event `SR_AddGreen`
  (`self.MC_AddGreen`))

(event `MC_AddGreen`
  (`/Engine/EditorBlueprintResources/StandardMacros.IncrementInt` (`/Game/_Framework/Blueprints/GS_Case.GreenToolAmount` (`self.GS`))))

(event `MC_AddYellow`
  (`/Engine/EditorBlueprintResources/StandardMacros.IncrementInt` (`/Game/_Framework/Blueprints/GS_Case.YellowToolAmount` (`self.GS`))))

(event `SR_AddYellow`
  (`self.MC_AddYellow`))

(fn `UserConstructionScript`)